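; BP_Canvas is a paintable canvas actor that stamps brush textures onto a runtime render target.
; On BeginPlay it creates and clears the render target, feeds it into a dynamic material on the Canvas component, and creates a dynamic brush material.
; DrawBrush sets the brush texture, then draws that material into the render target, centered on a normalized location at the given size.
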(event `self.ReceiveBeginPlay`
  (`|ExecutionSequence`
    (:`then_0`
      (bind _returnvalue (`KismetRenderingLibrary.CreateRenderTarget2D` 1024 1024))
      (bind _output_get (set `self.RenderTarget` _returnvalue))
      (`KismetRenderingLibrary.ClearRenderTarget2D` _output_get (struct :`R` 255.0 :`G` 255.0 :`B` 255.0 :`A` 1.0)))
    (:`then_1`
      (bind _returnvalue_2 (`KismetMaterialLibrary.CreateDynamicMaterialInstance` null))
      (`MaterialInstanceDynamic.SetTextureParameterValue` _returnvalue_2 "RenderTarget" (`self.RenderTarget`))
      (`PrimitiveComponent.SetMaterial` (`self.Canvas`) 0 _returnvalue_2))
    (:`then_2`
      (bind _returnvalue_3 (`KismetMaterialLibrary.CreateDynamicMaterialInstance` null))
      (set `self.BrushMaterial` _returnvalue_3))))

(fn `DrawBrush`
  (params (brushtexture :type "Texture2D Object Reference") (brushsize :type "Float (double-precision)") (drawlocation :type "Vector2D Structure"))
  (bind _brushsize (`local.brushsize`))
  (`|ExecutionSequence`
    (:`then_0`
      (`MaterialInstanceDynamic.SetTextureParameterValue` (`self.BrushMaterial`) "brushtexture" brushtexture))
    (:`then_1`
      (bind (_canvas _size _context) (`KismetRenderingLibrary.BeginDrawCanvasToRenderTarget` (`self.RenderTarget`)))
      (`Canvas.K2_DrawMaterial` _canvas (`self.BrushMaterial`) (- (* _size (`local.drawlocation`)) (/ _brushsize 2.0)) (`KismetMathLibrary.MakeVector2D` _brushsize _brushsize) (0.0 0.0) (1.0 1.0) 0.0 (0.5 0.5))
      (`KismetRenderingLibrary.EndDrawCanvasToRenderTarget` _context))))

(fn `UserConstructionScript`)